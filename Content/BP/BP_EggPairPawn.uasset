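; BP_EggPairPawn is a pawn that rolls two physics eggs, each driven by its own movement input.
; It adds the IMC_EggPair mapping context on BeginPlay and stores both input vectors.
; Each Tick centers the actor between the eggs and applies actor-relative torque above a deadzone, with opposite Y signs per egg.
; Helper names are swapped: HandleRightEgg drives EggLeft from MoveLeft, and HandleLeftEgg drives EggRight.
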(event `EnhancedInput|/Game/Input/IA_MoveLeft`
  (params (ActionValue :type "Vector2D Structure") (ElapsedSeconds :type "Float (double-precision)") (TriggeredSeconds :type "Float (double-precision)") (InputAction :type "InputAction Object Reference" :default "/Game/Input/IA_MoveLeft.IA_MoveLeft"))
  (:`Triggered`
    (set `self.MoveLeft` ActionValue)))

(event `EnhancedInput|/Game/Input/IA_MoveRight`
  (params (ActionValue :type "Vector2D Structure") (ElapsedSeconds :type "Float (double-precision)") (TriggeredSeconds :type "Float (double-precision)") (InputAction :type "InputAction Object Reference" :default "/Game/Input/IA_MoveRight.IA_MoveRight"))
  (:`Triggered`
    (set `self.MoveRight` ActionValue)))

(event `self.ReceiveBeginPlay`
  (`KismetSystemLibrary.PrintString` "Egg Pawn Begin Play")
  (`EnhancedInputSubsystemInterface.AddMappingContext` (pcsubsystem `EnhancedInputLocalPlayerSubsystem` (`GameplayStatics.GetPlayerController` 0)) "/Game/Input/IMC_EggPair.IMC_EggPair" 0 (struct)))

(event `self.ReceiveTick`
  (params (DeltaSeconds :type "Float (single-precision)"))
  (bind _torquestrength (`self.TorqueStrength`))
  (`self.K2_SetActorLocation` (* (+ (`SceneComponent.K2_GetComponentLocation` (`self.EggLeft`)) (`SceneComponent.K2_GetComponentLocation` (`self.EggRight`))) 0.5))
  (`self.HandleRightEgg` (`self.MoveLeft`) _torquestrength)
  (`self.HandleLeftEgg` (`self.MoveRight`) _torquestrength))

(fn `HandleLeftEgg`
  (params (MoveRight2DVector :type "Vector2D Structure") (TorqueStr :type "Float (double-precision)"))
  (bind (_x _y) (`KismetMathLibrary.BreakVector2D` MoveRight2DVector))
  (if (> (`KismetMathLibrary.VSize2D` MoveRight2DVector) 0.2)
    (`PrimitiveComponent.AddTorqueInRadians` (`self.EggRight`) (* (+ (* (* _x -1.0) (`self.GetActorRightVector`)) (* (`self.GetActorForwardVector`) (* _y -1.0))) TorqueStr) "None" true)))

(fn `HandleRightEgg`
  (params (MoveLeft2DVector :type "Vector2D Structure") (TorqueStr :type "Float (double-precision)"))
  (bind (_x _y) (`KismetMathLibrary.BreakVector2D` MoveLeft2DVector))
  (if (> (`KismetMathLibrary.VSize2D` MoveLeft2DVector) 0.2)
    (`PrimitiveComponent.AddTorqueInRadians` (`self.EggLeft`) (* (+ (* (* _x -1.0) (`self.GetActorRightVector`)) (* (* _y 1.0) (`self.GetActorForwardVector`))) TorqueStr) "None" true)))

(fn `UserConstructionScript`)